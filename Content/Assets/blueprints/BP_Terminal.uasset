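; Interactable terminal that maps a 7x7 inventory onto a world grid of rooms around itself.
; BeginPlay spawns 49 BP_Empty_Room actors at fixed offsets and, after short delays, a matching player-linked BP_Invintory seeded with three BP_BASE items.
; UpdateRooms sets each room from the item in the same-index slot.
; Interact refreshes the inventory slots, while ShowE and HideE toggle the interaction prompt.
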(event `self.ReceiveBeginPlay`
  (bind _returnvalue_location (`KismetMathLibrary.BreakTransform` (`self.GetTransform`)))
  ;[1 1 1] begin Play
  (`|ExecutionSequence`
    (:`then_0`
      (bind _asbp_player_ (cast `/Game/Assets/blueprints/Player/BP_Player_` (`GameplayStatics.GetPlayerCharacter` 0))
        (:`then`
          (`KismetSystemLibrary.Delay` 0.01)
          (if (`KismetSystemLibrary.IsValid` (`/Game/Assets/blueprints/BP_Invintory.Main Widget` (`/Game/Assets/blueprints/Player/BP_Player_.Invintory Ref` _asbp_player_)))
            (bind _returnvalue (`|SpawnActorFromClass` "/Game/Assets/blueprints/BP_Invintory.BP_Invintory_C" (`KismetMathLibrary.MakeTransform` (0.0 0.0 0.0)) "AlwaysSpawn" "MultiplyWithRoot" null 49 1 _asbp_player_ 7 true null))
            (bind _output_get (set `self.Invintory Ref` _returnvalue))
            (`KismetSystemLibrary.Delay` 0.01)
            (`/Game/Assets/blueprints/BP_Invintory.AddItemAtIndex` _output_get "/Game/Assets/blueprints/Items_Tiles/BP_BASE.BP_BASE_C" 1 24)
            (`/Game/Assets/blueprints/BP_Invintory.AddItemAtIndex` _output_get "/Game/Assets/blueprints/Items_Tiles/BP_BASE.BP_BASE_C" 1 3)
            (`/Game/Assets/blueprints/BP_Invintory.AddItemAtIndex` _output_get "/Game/Assets/blueprints/Items_Tiles/BP_BASE.BP_BASE_C" 1 48)
            (`self.Update Rooms`)))
        (:`CastFailed`
          (`KismetSystemLibrary.PrintString` "Player Cast Failed" true true (struct :`R` 1.0 :`G` 0.026519 :`A` 1.0)))))
    (:`then_1`
      (for _index (range 49)
        (bind _returnvalue_2 (`|SpawnActorFromClass` "/Game/Assets/blueprints/Rooms/BP_Empty_Room.BP_Empty_Room_C" (`KismetMathLibrary.MakeTransform` (+ _returnvalue_location (select `int` _index :`0` (-5400.0 5400.0 -75.0) :`1` (-5400.0 3600.0 -75.0) :`2` (-5400.0 1800.0 -75.0) :`3` (-5400.0 0.0 -75.0) :`4` (-5400.0 -1800.0 -75.0) :`5` (-5400.0 -3600.0 -75.0) :`6` (-5400.0 -5400.0 -75.0) :`7` (-3600.0 5400.0 -75.0) :`8` (-3600.0 3600.0 -75.0) :`9` (-3600.0 1800.0 -75.0) :`10` (-3600.0 0.0 -75.0) :`11` (-3600.0 -1800.0 -75.0) :`12` (-3600.0 -3600.0 -75.0) :`13` (-3600.0 -5400.0 -75.0) :`14` (-1800.0 5400.0 -75.0) :`15` (-1800.0 3600.0 -75.0) :`16` (-1800.0 1800.0 -75.0) :`17` (-1800.0 0.0 -75.0) :`18` (-1800.0 -1800.0 -75.0) :`19` (-1800.0 -3600.0 -75.0) :`20` (-1800.0 -5400.0 -75.0) :`21` (0.0 5400.0 -75.0) :`22` (0.0 3600.0 -75.0) :`23` (0.0 1800.0 -75.0) :`24` (0.0 0.0 -75.0) :`25` (0.0 -1800.0 -75.0) :`26` (0.0 -3600.0 -75.0) :`27` (0.0 -5400.0 -75.0) :`28` (1800.0 5400.0 -75.0) :`29` (1800.0 3600.0 -75.0) :`30` (1800.0 1800.0 -75.0) :`31` (1800.0 0.0 -75.0) :`32` (1800.0 -1800.0 -75.0) :`33` (1800.0 -3600.0 -75.0) :`34` (1800.0 -5400.0 -75.0) :`35` (3600.0 5400.0 -75.0) :`36` (3600.0 3600.0 -75.0) :`37` (3600.0 1800.0 -75.0) :`38` (3600.0 0.0 -75.0) :`39` (3600.0 -1800.0 -75.0) :`40` (3600.0 -3600.0 -75.0) :`41` (3600.0 -5400.0 -75.0) :`42` (5400.0 5400.0 -75.0) :`43` (5400.0 3600.0 -75.0) :`44` (5400.0 1800.0 -75.0) :`45` (5400.0 0.0 -75.0) :`46` (5400.0 -1800.0 -75.0) :`47` (5400.0 -3600.0 -75.0) :`48` (5400.0 -5400.0 -75.0) :!type "Vector Structure"))) "Undefined" "MultiplyWithRoot" null null))
        (`KismetArrayLibrary.Array_Add` (`self.empty rooms`) _returnvalue_2)))))

(event `Update Rooms`
  (for (_array_element _array_index) (`self.empty rooms`)
    (`/Game/Assets/blueprints/Rooms/BP_Empty_Room.Set Room` _array_element (`.Room_27_1A97E0E94E31A8D478C295A58BA0870F` (break `/Game/Assets/blueprints/Fundementals/S_ItemInfo` (`.ItemInfo` (`/Game/Assets/blueprints/BP_Invintory.GetItemInfoAtIndex` (`self.Invintory Ref`) _array_index)))))))

(event `/Game/Assets/blueprints/Fundementals/IN_Interact_Interface.Interact`
  (params (`Terminal Widget` :type "/Game/Assets/UI/Widgets/TerminalWidget Object Reference"))
  (for (_ _array_index) (`/Game/Assets/blueprints/BP_Invintory.Slots` (`self.Invintory Ref`))
    (`/Game/Assets/blueprints/BP_Invintory.UpdateSlotAtIndex` (`self.Invintory Ref`) _array_index)))

(event `Show E`
  (`SceneComponent.SetHiddenInGame` (`self.interact_E`) false false))

(event `Hide E`
  (`SceneComponent.SetHiddenInGame` (`self.interact_E`) true false))

(fn `UserConstructionScript`)