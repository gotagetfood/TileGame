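; Slot-based inventory Blueprint that stores items as class and amount pairs in an array sized on BeginPlay.
; Helper functions find empty slots or partial stacks and read item info from class defaults.
; AddItem recursively spreads items over stacks or single slots, returning false only if the first placement fails.
; As written, stack overflow re-adds AmountOfSlots instead of the remainder, and new stacks always get MaxStackSize.
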(event `self.ReceiveBeginPlay`
  ;[1 1 1] slots
  (`KismetArrayLibrary.Array_Resize` (`self.Slots`) (`self.AmountOfSlots`)))

(fn `AddItem`
  (params (itemclass :type "/Game/Assets/blueprints/Items_Tiles/BP_MasterTile Class Reference") (amount :type Integer))
  (returns (`Success?` :type Boolean))
  (locals (`local class` :type "/Game/Assets/blueprints/Items_Tiles/BP_MasterTile Class Reference") (`local amount` :type Integer) (`Local Index` :type Integer :default 0))
  (bind _returnvalue (+ (`.Amount_5_4A8DBBBC44708A3261D7569189E76A01` (break `/Game/Assets/blueprints/Structures/S_InvintorySlot` (`|GetArrayItem` (`self.Slots`) (`local.Local Index`)))) (`local.local amount`)))
  (set `local.local class` itemclass)
  (set `local.local amount` amount)
  (if (`.CanBeStacked?_19_C56F64234285813315868CB029AE0EA8` (break `/Game/Assets/blueprints/Structures/S_ItemInfo` (defaults `Object` itemclass)))
    ;[1 1 1] stackable
    (bind (_success_ _index) (`self.SearchFreeStack` (`local.local class`)))
    (if _success_
      (set `local.Local Index` _index)
      (if (> _returnvalue (`self.MaxStackSize`))
        (set `local.local amount` (- _returnvalue (`self.MaxStackSize`)))
        (`KismetArrayLibrary.Array_Set` (`self.Slots`) (`local.Local Index`) (make `/Game/Assets/blueprints/Structures/S_InvintorySlot` (`local.local class`) (`self.MaxStackSize`)))
        (`self.AddItem` (`local.local class`) (`self.AmountOfSlots`))
        (return true)
        (else
          (`KismetArrayLibrary.Array_Set` (`self.Slots`) (`local.Local Index`) (make `/Game/Assets/blueprints/Structures/S_InvintorySlot` (`local.local class`) _returnvalue))
          (return true)))
      (else
        (bind (_success__2 _index_2) (`self.SearchEmptySlot`))
        (if _success__2
          (set `local.Local Index` _index_2)
          (if (> (`local.local amount`) (`self.MaxStackSize`))
            (`KismetArrayLibrary.Array_Set` (`self.Slots`) (`local.Local Index`) (make `/Game/Assets/blueprints/Structures/S_InvintorySlot` (`local.local class`) (`self.MaxStackSize`)))
            (`self.AddItem` (`local.local class`) (- (`local.local amount`) (`self.MaxStackSize`)))
            (return true)
            (else
              (`KismetArrayLibrary.Array_Set` (`self.Slots`) (`local.Local Index`) (make `/Game/Assets/blueprints/Structures/S_InvintorySlot` (`local.local class`) (`self.MaxStackSize`)))
              (return true)))
          (else
            (return false)))))
    (else
      ;[1 1 1] unstackables
      (bind (_success__3 _index_3) (`self.SearchEmptySlot`))
      (if _success__3
        (bind _output_get (set `local.Local Index` _index_3))
        (`KismetArrayLibrary.Array_Set` (`self.Slots`) _output_get (make `/Game/Assets/blueprints/Structures/S_InvintorySlot` (`local.local class`) 1))
        (if (> (`local.local amount`) 1)
          (`self.AddItem` (`local.local class`) (- (`local.local amount`) 1))
          (return true)
          (else
            (return true)))
        (else
          (return false))))))

(fn `GetItemInfoAtIndex`
  (params (Index :type Integer))
  (returns (`EmptySlot?` :type Boolean) (ItemInfo :type "/Game/Assets/blueprints/Structures/S_ItemInfo Structure") (Amount :type Integer))
  (bind (_itemclass _amount) (break `/Game/Assets/blueprints/Structures/S_InvintorySlot` (`|GetArrayItem` (`self.Slots`) Index)))
  (if (`KismetSystemLibrary.IsValidClass` _itemclass)
    (return false (defaults `Object` _itemclass) _amount)
    (else
      (return true (struct) 0))))

(fn `IsSlotEmpty`
  (params (index :type Integer))
  (returns (`Empty?` :type Boolean))
  (return (not (`KismetSystemLibrary.IsValidClass` (`.ItemClass_3_CEE27CF34BF4950897B3A48120F93CC9` (break `/Game/Assets/blueprints/Structures/S_InvintorySlot` (`|GetArrayItem` (`self.Slots`) index)))))))

(fn `SearchEmptySlot`
  (returns (`Success?` :type Boolean) (index :type Integer))
  (locals (LocalBool :type Boolean) (LocalIndex :type Integer))
  (for (_array_element _array_index) (`self.Slots`)
    (if (not (`KismetSystemLibrary.IsValidClass` (`.ItemClass_3_CEE27CF34BF4950897B3A48120F93CC9` (break `/Game/Assets/blueprints/Structures/S_InvintorySlot` _array_element))))
      (set `local.LocalBool` true)
      (set `local.LocalIndex` _array_index)
      (break)))
  (return (`local.LocalBool`) (`local.LocalIndex`)))

(fn `SearchFreeStack`
  (params (`Item Class` :type "/Game/Assets/blueprints/Items_Tiles/BP_MasterTile Class Reference"))
  (returns (`Success?` :type Boolean) (index :type Integer))
  (locals (localbool :type Boolean) (localindex :type Integer))
  (for (_array_element _array_index) (`self.Slots`)
    (bind (_itemclass _amount) (break `/Game/Assets/blueprints/Structures/S_InvintorySlot` _array_element))
    (if (`KismetSystemLibrary.IsValidClass` _itemclass)
      (if (and (== _itemclass `Item Class`) (< _amount (`self.MaxStackSize`)))
        (set `local.localindex` _array_index)
        (set `local.localbool` true)
        (break))))
  (return (`local.localbool`) (`local.localindex`)))

(fn `UserConstructionScript`)