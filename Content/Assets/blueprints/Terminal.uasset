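; Interactable terminal actor that shows a prompt when the player is near and opens a widget on interaction.
; AreaBox overlap events, filtered to BP_Player_, unhide and hide the InteractE prompt.
; The Interact event prints a debug message, then calls Show on the widget passed to it unless that widget is already in the viewport.
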(event `self.Area Box.OnComponentBeginOverlap`
  (params (OverlappedComponent :type "PrimitiveComponent Object Reference") (OtherActor :type "Actor Object Reference") (OtherComp :type "PrimitiveComponent Object Reference") (OtherBodyIndex :type Integer) (bFromSweep :type Boolean) (SweepResult :type "HitResult Structure (by ref)"))
  (cast `/Game/Assets/blueprints/Player/BP_Player_` OtherActor)
  (`SceneComponent.SetHiddenInGame` (`self.interact_E`) false false))

(event `self.Area Box.OnComponentEndOverlap`
  (params (OverlappedComponent :type "PrimitiveComponent Object Reference") (OtherActor :type "Actor Object Reference") (OtherComp :type "PrimitiveComponent Object Reference") (OtherBodyIndex :type Integer))
  (cast `/Game/Assets/blueprints/Player/BP_Player_` OtherActor)
  (`SceneComponent.SetHiddenInGame` (`self.interact_E`) true false))

(event `/Game/Assets/blueprints/Fundementals/IN_Interact_Interface.Interact`
  (params (Widget :type "/Game/Assets/UI/Old/Termnal_Widget Object Reference"))
  (`KismetSystemLibrary.PrintString` "Interacted")
  (if (not (`Widget.IsInViewport` Widget))
    (`/Game/Assets/UI/Old/Termnal_Widget.Show` Widget "E")))

(fn `UserConstructionScript`)