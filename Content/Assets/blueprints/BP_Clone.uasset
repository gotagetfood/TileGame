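; BP_Clone is an interactable respawn point that sets the player's SpawnPoint to the world location of its Arrow component.
; Interact performs the update, and an instance flagged StartingSpawn also does so on BeginPlay after a very short delay.
; ShowE and HideE toggle the InteractE prompt's visibility.
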(event `self.ReceiveBeginPlay`
  (if (`self.StartingSpawn?`)
    (`KismetSystemLibrary.Delay` 0.01)
    (bind _asbp_player_ (cast `/Game/Assets/blueprints/Player/BP_Player_` (`GameplayStatics.GetPlayerCharacter` 0) :!label _label))
    (set `/Game/Assets/blueprints/Player/BP_Player_.SpawnPoint` (`SceneComponent.K2_GetComponentLocation` (`self.Arrow`)) _asbp_player_)))

(event `/Game/Assets/blueprints/Fundementals/IN_Interact_Interface.Interact`
  (params (`Terminal Widget` :type "/Game/Assets/UI/Widgets/TerminalWidget Object Reference"))
  (goto _label))

(event `Show E`
  (`SceneComponent.SetHiddenInGame` (`self.interact_E`) false false))

(event `Hide E`
  (`SceneComponent.SetHiddenInGame` (`self.interact_E`) true false))

(fn `UserConstructionScript`)