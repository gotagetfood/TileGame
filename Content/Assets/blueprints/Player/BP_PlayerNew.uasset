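; Player character that shows a sprite in a 3D world, with axis movement, jump and sprint, which changes walk speed and animation play rate.
; Each tick it derives a facing direction enum from input, favoring horizontal, and flips the sprite by setting its world yaw for two directions.
; Overlaps trigger pickups through Collect_Interface, and the Interact input messages the first overlapping Interact_Interface actor.
; Construction tilts the sprite by half the spring arm pitch.
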(event `self.ReceiveActorBeginOverlap`
  (params (OtherActor :type "Actor Object Reference"))
  ;[1 1 1] pick up
  (if (`KismetSystemLibrary.DoesImplementInterface` OtherActor "/Game/Assets/blueprints/Collect_Interface.Collect_Interface_C")
    (message `/Game/Assets/blueprints/Collect_Interface.Pick Up` OtherActor)))

(event `self.ReceiveTick`
  (params (DeltaSeconds :type "Float (single-precision)"))
  (`|ExecutionSequence`
    (:`then_0`
      ;[1 1 1] Animation Stuff
      (`self.Set Direction`)
      (`self.Set Flip`))))

(event `InputAxis|Move Up`
  (params (AxisValue :type "Float (single-precision)"))
  ;[1 1 1] Controls
  (`self.AddMovementInput` (-1.0 0.0 0.0) AxisValue))

(event `InputAxis|Move Right`
  (params (AxisValue :type "Float (single-precision)"))
  ;[1 1 1] Controls
  (`self.AddMovementInput` (0.0 -1.0 0.0) AxisValue))

(event `InputAction|Jump`
  (params (Key :type "Key Structure"))
  ;[1 1 1] Controls
  (:`Pressed`
    (`self.Jump`))
  (:`Released`
    (`self.StopJumping`)))

(event `InputAction|Sprint`
  (params (Key :type "Key Structure"))
  (bind _charactermovement (`self.CharacterMovement`))
  ;[1 1 1] Controls
  (:`Pressed`
    (set `CharacterMovementComponent.MaxWalkSpeed` 1200.0 _charactermovement)
    (set `self.Run_PlayRate` 1.5))
  (:`Released`
    (set `CharacterMovementComponent.MaxWalkSpeed` 800.0 _charactermovement)
    (set `self.Run_PlayRate` 1.0)))

(event `InputAction|Interact`
  (params (Key :type "Key Structure"))
  ;[1 1 1] Controls
  (:`Pressed`
    (for _array_element (`self.GetOverlappingActors` null)
      (if (`KismetSystemLibrary.DoesImplementInterface` _array_element "/Game/Assets/blueprints/Interact_Interface.Interact_Interface_C")
        (message `/Game/Assets/blueprints/Interact_Interface.Interact` _array_element)
        (break)))))

(fn `Set Direction`
  ;[1 1 1] get current state
  (if (or (!= (`self.GetInputAxisValue`) 0.0) (!= (`self.GetInputAxisValue`) 0.0))
    (set `self.direction` (select `bool` (> (`self.GetInputAxisValue`) 0.0) :`false` (select `bool` (< (`self.GetInputAxisValue`) 0.0) :`false` (select `bool` (> (`self.GetInputAxisValue`) 0.0) :`false` "NewEnumerator1" :`true` "NewEnumerator0" :!type "/Game/Assets/blueprints/Direction Enum") :`true` "NewEnumerator3") :`true` "NewEnumerator2"))))

(fn `Set Flip`
  (bind _sprite (`self.Sprite`))
  (`|ExecutionSequence`
    (:`then_0`
      ;[1 1 1] Set Rotation
      (if (== (`self.direction`) 2)
        (`SceneComponent.K2_SetWorldRotation` _sprite (`KismetMathLibrary.MakeRotator` 0.0 0.0 -90.0) false false)))
    (:`then_1`
      (if (== (`self.direction`) 3)
        (`SceneComponent.K2_SetWorldRotation` _sprite (`KismetMathLibrary.MakeRotator` 0.0 0.0 90.0) false false)))))

(fn `UserConstructionScript`
  (bind (_returnvalue_roll _returnvalue_pitch) (`KismetMathLibrary.BreakRotator` (`SceneComponent.K2_GetComponentRotation` (`self.SpringArm`))))
  (`SceneComponent.K2_SetWorldRotation` (`self.Sprite`) (`KismetMathLibrary.MakeRotator` (/ _returnvalue_pitch 2.0) 0.0 -90.0) false false))