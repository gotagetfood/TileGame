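; BP_Exit is an interactable exit that brings up the end screen for the player.
; Interact shows the mouse cursor, switches input to UI only and makes the EndScreen visible through the player's inventory main widget.
; When StartingSpawn is set, BeginPlay runs the same sequence after a very short delay.
; ShowE and HideE toggle the InteractE prompt.
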(event `self.ReceiveBeginPlay`
  (bind _returnvalue (`GameplayStatics.GetPlayerController` 0))
  (if (`self.StartingSpawn?`)
    (`KismetSystemLibrary.Delay` 0.01)
    (bind _asbp_player_ (cast `/Game/Assets/blueprints/Player/BP_Player_` (`GameplayStatics.GetPlayerCharacter` 0) :!label _label))
    (set `PlayerController.bShowMouseCursor` true _returnvalue)
    (`WidgetBlueprintLibrary.SetInputMode_UIOnlyEx` _returnvalue null "DoNotLock" true)
    (`/Game/Assets/UI/Widgets/EndScreen.Set Visible` (`/Game/Assets/UI/Widgets/MainWidget.EndScreen` (`/Game/Assets/blueprints/BP_Invintory.Main Widget` (`/Game/Assets/blueprints/Player/BP_Player_.Invintory Ref` _asbp_player_))))))

(event `/Game/Assets/blueprints/Fundementals/IN_Interact_Interface.Interact`
  (params (`Terminal Widget` :type "/Game/Assets/UI/Widgets/TerminalWidget Object Reference"))
  (goto _label))

(event `Show E`
  (`SceneComponent.SetHiddenInGame` (`self.interact_E`) false false))

(event `Hide E`
  (`SceneComponent.SetHiddenInGame` (`self.interact_E`) true false))

(fn `UserConstructionScript`)