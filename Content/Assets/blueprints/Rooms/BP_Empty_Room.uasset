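; BP_Empty_Room is a placeholder actor that hosts one swappable room at its own location.
; The SetRoom event passes a room class to the Set Room function, which destroys any valid current room, spawns the new class at the actor's transform and stores it.
; BeginPlay is empty, and a leftover random pick among six room Blueprints is disconnected, so it never runs.
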(event `Set Room`
  (params (`Room ITem` :type "/Game/Assets/blueprints/Rooms/BP_Room_BASE Class Reference"))
  ;[1 1 1] Comment
  (`self.Set Room` `Room ITem`))

(event `self.ReceiveBeginPlay`)

(fn `Set Room`
  (params (NewParam :type "/Game/Assets/blueprints/Rooms/BP_Room_BASE Class Reference"))
  (bind _room (`self.Room`))
  (if (`KismetSystemLibrary.IsValid` _room)
    (`self.K2_DestroyActor` _room))
  (bind _returnvalue (`|SpawnActorFromClass` NewParam (`self.GetTransform`) "Undefined" "MultiplyWithRoot" null null))
  (set `self.Room` _returnvalue))

(fn `UserConstructionScript`)