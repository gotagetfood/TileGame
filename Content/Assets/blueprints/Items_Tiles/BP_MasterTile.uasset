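; BP_MasterTile is a pickup item actor that spins, bobs and adds its item to an inventory when picked up.
; BeginPlay sets the RotatingMovement rate from RotateSpeed plus a random offset, and Tick applies a sine-driven vertical offset scaled by Speed and Distance.
; PickUp calls PickedUp, which prints the item name, calls AddItem on a valid inventory, then on success keeps any leftover Amount or destroys the actor.
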(event `self.ReceiveTick`
  (params (DeltaSeconds :type "Float (single-precision)"))
  ;[1 1 1] Rotations
  (`self.K2_AddActorWorldOffset` (`KismetMathLibrary.MakeVector` 0.0 0.0 (* 1.0 (* (* (`KismetMathLibrary.DegSin` (* (`self.GetGameTimeSinceCreation`) (`self.Speed`))) 0.01111) (`self.distance`))))))

(event `self.ReceiveBeginPlay`
  ;[1 1 1] Rotations
  (set `RotatingMovementComponent.RotationRate` (`KismetMathLibrary.MakeRotator` 0.0 0.0 (+ (`self.Rotate Speed`) (`KismetMathLibrary.RandomFloatInRange` -10.0 10.0))) (`self.RotatingMovement`)))

(event `/Game/Assets/blueprints/Fundementals/IN_Collect_Interface.Pick Up`
  (params (`Invintory Ref` :type "/Game/Assets/blueprints/BP_Invintory Object Reference"))
  (`self.Picked Up` `Invintory Ref`))

(event `EventOnUsed`)

(fn `Picked Up`
  (params (`Invintory Ref` :type "/Game/Assets/blueprints/BP_Invintory Object Reference"))
  (`KismetSystemLibrary.PrintString` (`KismetTextLibrary.Conv_TextToString` (`.Name_16_70887EF14EE7B5A4BA9B7AB391384DE4` (break `/Game/Assets/blueprints/Fundementals/Structures/S_ItemInfo` (`self.ItemInfo`)))))
  (`/Engine/EditorBlueprintResources/StandardMacros.IsValid` `Invintory Ref`
    (:`Is Valid`
      (bind (_success_ _rest) (`/Game/Assets/blueprints/BP_Invintory.AddItem` `Invintory Ref` (`self.ItemToAdd`) (`self.Amount`)))
      (if _success_
        (if (> _rest 0)
          (set `self.Amount` _rest)
          (else
            (`self.K2_DestroyActor`)))))))

(fn `UserConstructionScript`)