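; BP_TileBase is a base tile item that spins and bobs in the world until picked up.
; BeginPlay sets the RotatingMovement yaw rate from RotateSpeed.
; Tick adds a vertical offset from a sine of time since creation, scaled by Speed and Distance, without delta time.
; PickedUp prints the ThumbNail object's name and destroys the actor.
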(event `self.ReceiveTick`
  (params (DeltaSeconds :type "Float (single-precision)"))
  (`self.K2_AddActorWorldOffset` (`KismetMathLibrary.MakeVector` 0.0 0.0 (* 1.0 (* (* (`KismetMathLibrary.DegSin` (* (`self.GetGameTimeSinceCreation`) (`self.Speed`))) 0.01111) (`self.distance`))))))

(event `self.ReceiveBeginPlay`
  (set `RotatingMovementComponent.RotationRate` (`KismetMathLibrary.MakeRotator` 0.0 0.0 (`self.Rotate Speed`)) (`self.RotatingMovement`)))

(fn `Picked_Up`
  (`KismetSystemLibrary.PrintString` (`KismetSystemLibrary.GetObjectName` (`self.ThumbNail`)))
  (`self.K2_DestroyActor`))

(fn `UserConstructionScript`)