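; Base enemy character with a sprite, providing shared facing, jump and death behavior.
; Each tick derives a four-way Direction from the move axes, favoring horizontal, yaws the sprite for two of those directions, and updates the on-ground flag.
; Death sets IsDead, then destroys the actor after a short delay.
; G and P keys trigger jump and death directly; damage and overlap handlers are empty stubs.
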(event `Key|G`
  (params (Key :type "Key Structure"))
  (:`Pressed`
    (`self.Jump`))
  (:`Released`
    (`self.StopJumping`)))

(event `self.ReceiveBeginPlay`
  ;[1 1 1] start up
)

(event `self.ReceiveTick`
  (params (DeltaSeconds :type "Float (single-precision)"))
  (`|ExecutionSequence`
    (:`then_0`
      ;[1 1 1] Animation Stuff
      (`self.Set Direction`)
      (`self.Set Flip`))
    (:`then_1`
      (set `self.isonGound?` (not (`NavMovementComponent.IsFalling` (`self.CharacterMovement`)))))))

(event `self.ReceiveActorBeginOverlap`
  (params (OtherActor :type "Actor Object Reference"))
  ;[1 1 1] overlap with picks and interacts
  (`|ExecutionSequence`))

(event `Key|P`
  (params (Key :type "Key Structure"))
  ;[1 1 1] Death
  (:`Pressed`
    (`self.Death`)))

(event `Death`
  ;[1 1 1] Death
  (set `self.isDead?` true)
  (`KismetSystemLibrary.Delay` 0.5)
  (`self.K2_DestroyActor`))

(event `/Game/Assets/blueprints/Fundementals/IN_Damage_interface.Damage It`
  (params (`Damage Delt` :type Integer)))

(fn `Set Direction`
  ;[1 1 1] get current state
  (if (or (!= (`self.GetInputAxisValue`) 0.0) (!= (`self.GetInputAxisValue`) 0.0))
    (set `self.direction` (select `bool` (> (`self.GetInputAxisValue`) 0.0) :`false` (select `bool` (< (`self.GetInputAxisValue`) 0.0) :`false` (select `bool` (> (`self.GetInputAxisValue`) 0.0) :`false` "NewEnumerator1" :`true` "NewEnumerator0" :!type "/Game/Assets/blueprints/Fundementals/E_Direction Enum") :`true` "NewEnumerator3") :`true` "NewEnumerator2"))))

(fn `Set Flip`
  (bind _sprite (`self.Sprite`))
  (`|ExecutionSequence`
    (:`then_0`
      ;[1 1 1] Set Rotation
      (if (== (`self.direction`) 2)
        (`SceneComponent.K2_SetWorldRotation` _sprite (`KismetMathLibrary.MakeRotator` 0.0 0.0 -90.0) false false)))
    (:`then_1`
      (if (== (`self.direction`) 3)
        (`SceneComponent.K2_SetWorldRotation` _sprite (`KismetMathLibrary.MakeRotator` 0.0 0.0 90.0) false false)))))

(fn `UserConstructionScript`)